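; BP_Dummy is a damageable Blueprint that implements simple health and death, labeled as player damage logic.
; AnyDamage subtracts damage from CurrentHealth, clamps it to a small fixed range and prints the result for debugging.
; At zero health it sets IsDead, which blocks further damage, and disables its input from player controller 0.
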(event Game|Damage|EventAnyDamage
  (params (Damage :type Float%20%28single-precision%29) (DamageType :type Damage%20Type%20Object%20Reference) (InstigatedBy :type Controller%20Object%20Reference) (DamageCauser :type Actor%20Object%20Reference))
  ;[1 0.01509 0 0.5] Player Taking Damage and Death
  (if (not (Variables|Default|GetisDead))
    (bind _output_get (Variables|Default|SetCurrentHealth (Math|Float|Clamp(Float) (- (Variables|Default|GetCurrentHealth) Damage) 0.0 2.0)))
    (Development|PrintString (Utilities|String|ToString(Float) _output_get) true true "(R=0.041421,G=1.000000,B=0.000000,A=1.000000)")
    (if (== _output_get 0.0)
      (Variables|Default|SetisDead true)
      (Input|DisableInput (Game|GetPlayerController 0)))))

(fn ConstructionScript)